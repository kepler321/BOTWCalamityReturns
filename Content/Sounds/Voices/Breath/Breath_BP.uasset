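; Blueprint that manages the player's breathing voice audio for running and recovering states.
; Start events spawn 2D breath cues at random offsets, fade them in and set IsRunning or IsRecovering.
; Stop events fade the stored sound out and clear the flag, with running cleared after a short delay.
; IsRecoveringStoppable reports whether the recovery sound is still playing and not being destroyed.
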(event `OnBreathRunning_Event`
  (bind _returnvalue (`GameplayStatics.SpawnSound2D` "/Game/Sounds/Voices/Breath/BreathRunning_Cue.BreathRunning_Cue" 1.0 1.0 (`KismetMathLibrary.RandomFloatInRange` 0.0 13.0) null false false))
  (bind _output_get (set `self.BreathRunningActiveSound` _returnvalue))
  (`AudioComponent.FadeIn` _output_get 0.5 1.0 0.0 "Logarithmic")
  (set `self.IsRunning` true))

(event `OnStopBreathRunning_Event`
  (`AudioComponent.FadeOut` (`self.BreathRunningActiveSound`) 0.5 0.0 "Logarithmic")
  (`KismetSystemLibrary.Delay` 0.5)
  (set `self.IsRunning` false))

(event `OnBreathRecovering_Event`
  (bind _returnvalue (`GameplayStatics.SpawnSound2D` "/Game/Sounds/Voices/Breath/BreathRecovering_Cue.BreathRecovering_Cue" 1.0 1.0 (`KismetMathLibrary.RandomFloatInRange` 0.0 16.0) null))
  (bind _output_get (set `self.BreathRecoverActiveSound` _returnvalue))
  (`AudioComponent.FadeIn` _output_get 0.1 1.0 0.0 "Logarithmic")
  (set `self.IsRecovering` true))

(event `OnStopBreathRecovering_Event`
  (`AudioComponent.FadeOut` (`self.BreathRecoverActiveSound`) 0.5 0.0 "Logarithmic")
  (set `self.IsRecovering` false))

(fn `IsRecoveringStoppable`
  (returns (Stoppable :type Boolean))
  (bind _breathrecoveractivesound (`self.BreathRecoverActiveSound`))
  (if (`self.IsBeingDestroyed` _breathrecoveractivesound)
    (return false)
    (else
      (return (`AudioComponent.IsPlaying` _breathrecoveractivesound)))))

(fn `NewFunction`)