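; BP_NPC is a monster NPC Blueprint that drives the creature's vocal sounds, attached to its body.
; BeginPlay fades in fast breathing and starts a self-repeating grunt chain, in which each finished grunt schedules the next after a random delay.
; Tick polls BP_NPCController's sensing flag and uses a DoOnce to play one shout per detection, resetting when sensing is lost.
; The shout's finish event feeds back into the same delayed grunt chain.
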(event `OnAudioFinished_Event`
  (`KismetSystemLibrary.Delay` (`KismetMathLibrary.RandomFloatInRange` 3.0 15.0) :!label _label)
  (bind _returnvalue (`GameplayStatics.SpawnSoundAttached` "/Game/Sounds/Voices/Monster/Growl/MonsterGrunt_NoReverb_Cue.MonsterGrunt_NoReverb_Cue" (`self.Body`) "None" (0.0 0.0 0.0) (struct) "KeepRelativeOffset" false 0.25 1.0 0.0 "/Game/Sounds/Attenuation/MonsterGrowlChaseAttenuation1.MonsterGrowlChaseAttenuation1" "/Game/Sounds/Concurrency/PreventNewSoundConcurrency.PreventNewSoundConcurrency" false))
  (add `AudioComponent.OnAudioFinished` _returnvalue (delegate `OnAudioFinished_Event`)))

(event `self.ReceiveBeginPlay`
  (bind _returnvalue (`GameplayStatics.SpawnSoundAttached` "/Game/Sounds/Monster/MonsterBreathFast_Cue.MonsterBreathFast_Cue" (`self.Body`) "None" (0.0 0.0 0.0) (struct) "KeepRelativeOffset" false 0.75 1.0 0.0 "/Game/Sounds/Attenuation/MonsterBreathChaseAttenuation.MonsterBreathChaseAttenuation" null))
  (`AudioComponent.FadeIn` _returnvalue 5.0 1.0 0.0 "Linear")
  (goto _label))

(event `self.ReceiveTick`
  (params (DeltaSeconds :type "Float (single-precision)"))
  (bind _asbp_npccontroller (cast `/Game/BluePrints/AI/NPC/BP_NPCController` (`AIBlueprintHelperLibrary.GetAIController` self)))
  (if (`/Game/BluePrints/AI/NPC/BP_NPCController.Successfully Sensed` _asbp_npccontroller)
    (`/Engine/EditorBlueprintResources/StandardMacros.DoOnce` false :!label _label_2
      (:`Completed`
        (bind _returnvalue (`GameplayStatics.SpawnSoundAttached` "/Game/Sounds/Voices/Monster/Growl/MonsterShoutNoEcho01_Cue.MonsterShoutNoEcho01_Cue" (`self.Body`) "None" (0.0 0.0 0.0) (struct) "KeepRelativeOffset" false 1.0 1.0 0.0 "/Game/Sounds/Attenuation/MonsterGrowlChaseAttenuation1.MonsterGrowlChaseAttenuation1" "/Game/Sounds/Concurrency/PreventNewSoundConcurrency.PreventNewSoundConcurrency" false))
        (add `AudioComponent.OnAudioFinished` _returnvalue (delegate `OnAudioFinished_Event`))))
    (else
      (goto _label_2 :!via `Reset`))))

(fn `UserConstructionScript`)