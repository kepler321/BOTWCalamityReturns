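; AI controller for NPCs that runs the BT_NPC behavior tree for path patrolling and player detection.
; On BeginPlay it seeds the Blackboard with the pawn's patrol path looping and wait settings plus a starting direction, though a comment flags the BP_NPC cast as failing.
; AI Perception updates CanSeePlayer whenever the first-person character is sensed or lost.
; AIDisable detaches the controlled pawn from the controller.
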(event `AI Disable`
  (`Pawn.DetachFromControllerPendingDestroy` (`self.K2_GetPawn`)))

(event `self.ReceiveBeginPlay`
  (`self.RunBehaviorTree` "/Game/BluePrints/AI/NPC/BT_NPC.BT_NPC")
  ;[1 1 1] This Fails
  (bind _asbp_npc (cast `/Game/BluePrints/AI/NPC/BP_NPC` (`self.K2_GetPawn`)))
  (bind _output_get (set `self.MyPawn` _asbp_npc))
  (`BlackboardComponent.SetValueAsBool` (`AIBlueprintHelperLibrary.GetBlackboard` null) "PathLooping" (`/Game/BluePrints/AI/NPC/BP_PatrolPath.IsLooping` (`/Game/BluePrints/AI/NPC/BP_NPC.PatrolPath` _output_get)))
  (`BlackboardComponent.SetValueAsInt` (`AIBlueprintHelperLibrary.GetBlackboard` null) "Direction" 1)
  (`BlackboardComponent.SetValueAsFloat` (`AIBlueprintHelperLibrary.GetBlackboard` null) "WaitTime" (`/Game/BluePrints/AI/NPC/BP_PatrolPath.WaitTime` (`/Game/BluePrints/AI/NPC/BP_NPC.PatrolPath` (`self.MyPawn`)))))

(event `self.AIPerception.OnTargetPerceptionUpdated`
  (params (Actor :type "Actor Object Reference") (Stimulus :type "AIStimulus Structure"))
  (cast `/Game/FirstPerson/Blueprints/BP_FirstPersonCharacter` Actor)
  (bind _output_get (set `self.Successfully Sensed` (`.bSuccessfullySensed` (break `AIStimulus` Stimulus))))
  (`BlackboardComponent.SetValueAsBool` (`AIBlueprintHelperLibrary.GetBlackboard` null) "CanSeePlayer" _output_get))

(fn `UserConstructionScript`)